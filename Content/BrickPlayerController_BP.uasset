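; Player controller for a falling-brick puzzle that moves and rotates the controlled brick pawn on a grid.
; Left, Right and Down step one unit on press and repeat on looping timers while held.
; Each step runs cube-coordinate blocking and grid-limit checks before offsetting the pawn, with left along +X.
; Rotate turns each cube 90 degrees by remapping relative X/Y, without collision or bounds checks, and prints its name.
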(event `InputAction|Left`
  (params (Key :type "Key Structure"))
  (:`Pressed`
    (`self.LeftSideMovement`)
    (`KismetSystemLibrary.K2_SetTimer` null "LeftSideMovement" 0.1 true))
  (:`Released`
    (`KismetSystemLibrary.K2_ClearTimer` null "LeftSideMovement")))

(event `InputAction|Right`
  (params (Key :type "Key Structure"))
  (:`Pressed`
    (`self.RightSideMovement`)
    (`KismetSystemLibrary.K2_SetTimer` null "RightSideMovement" 0.1 true))
  (:`Released`
    (`KismetSystemLibrary.K2_ClearTimer` null "RightSideMovement")))

(event `InputAction|Down`
  (params (Key :type "Key Structure"))
  (:`Pressed`
    (`self.DownSideMovement`)
    (`KismetSystemLibrary.K2_SetTimer` null "DownSideMovement" 0.1 true))
  (:`Released`
    (`KismetSystemLibrary.K2_ClearTimer` null "DownSideMovement")))

(event `InputAction|Rotate`
  (params (Key :type "Key Structure"))
  (:`Pressed`
    (`self.RotateMovement`)))

(fn `DownSideMovement`
  (bind (_gridminxy_x _gridminxy_y) (`KismetMathLibrary.BreakVector2D` (`self.GridMinXY`)))
  (bind _returnvalue (`self.GetCubesCoordinates`))
  (`self.CheckForDownSide` _returnvalue)
  (bind _returnvalue_2 (`self.GetMinYCoordinate` _returnvalue))
  (if (and (not (`KismetMathLibrary.NearlyEqual_FloatFloat` _gridminxy_y _returnvalue_2 0.01)) (`self.IsAbleMoveDown`))
    (`self.K2_AddActorLocalOffset` (`self.K2_GetPawn`) (`KismetMathLibrary.MakeVector` 0.0 (* -1 (`self.UnitLength`))) false false)))

(fn `LeftSideMovement`
  (bind _gridmaxxy_x (`KismetMathLibrary.BreakVector2D` (`self.GridMaxXY`)))
  (bind _returnvalue (`self.GetCubesCoordinates`))
  (`self.CheckForLeftSide` _returnvalue)
  (bind _returnvalue_2 (`self.GetMaxXCoordinate` _returnvalue))
  (if (and (< _returnvalue_2 _gridmaxxy_x) (`self.IsAbleMoveLeft`))
    (`self.K2_AddActorLocalOffset` (`self.K2_GetPawn`) (`KismetMathLibrary.MakeVector` (`self.UnitLength`)) false false)
    (set `self.IsAbleMoveRight` true)))

(fn `RightSideMovement`
  (bind _gridminxy_x (`KismetMathLibrary.BreakVector2D` (`self.GridMinXY`)))
  (bind _returnvalue (`self.GetCubesCoordinates`))
  (`self.CheckForRightSide` _returnvalue)
  (bind _returnvalue_2 (`self.GetMinXCoordinate` _returnvalue))
  (if (and (> _returnvalue_2 _gridminxy_x) (`self.IsAbleMoveRight`))
    (`self.K2_AddActorLocalOffset` (`self.K2_GetPawn`) (`KismetMathLibrary.MakeVector` (* -1 (`self.UnitLength`))) false false)
    (set `self.IsAbleMoveLeft` true)))

(fn `RotateMovement`
  (for _array_element (`self.CubesMeshesForBrick`)
    (`KismetSystemLibrary.PrintString` (`KismetSystemLibrary.GetDisplayName` _array_element))
    (bind _returnvalue (`SceneComponent.GetRelativeTransform` _array_element))
    (`SceneComponent.K2_SetRelativeLocation` _array_element (`KismetMathLibrary.MakeVector` (* (.y (.location _returnvalue)) -1.0) (.x (.location _returnvalue))) false false)))

(fn `UserConstructionScript`)